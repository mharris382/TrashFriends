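; Player bear pawn that grabs, carries and throws spawnable physics objects, favoring the Dumpster as target.
; Grab takes the nearest overlapping BP_SpawnableBase, records its holder, and carries it on a PhysicsHandle.
; Throw applies doubled suggested-arc velocity toward the Dumpster if near or faced, otherwise straight ahead; empty-handed, it fires ImpactExecutor.
; Each tick aligns the camera rig and body pivot from the shared BP_Camera toward BP_CameraTarget.
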(event Input|EnhancedActionEvents|EnhancedInputActionIA_Grab
  (params (ActionValue :type Boolean) (ElapsedSeconds :type Float%20%28double-precision%29) (TriggeredSeconds :type Float%20%28double-precision%29) (InputAction :type Input%20Action%20Object%20Reference :default "/Game/ThirdPerson/Input/Actions/IA_Grab.IA_Grab"))
  (:Started
    (Utilities|HasGrabbed
      (:Has%20Grabbed
        (Physics|Components|PhysicsHandle|ReleaseComponent (Variables|Default|GetPhysicsHandle)))
      (:No%20Grabbed
        (bind (_canpickup _pickup) (CallFunction|GetGrabComponent))
        (if _canpickup
          (bind _output_get (Variables|Default|SetLastGrabbed _pickup))
          (Transformation|SetWorldLocation _output_get (Transformation|GetWorldLocation (Variables|Default|GetSphere)) false false)
          (Class|PhysicsHandleComponent|GrabComponentatLocation (Variables|Default|GetPhysicsHandle) _pickup "None" (Transformation|GetWorldLocation (Variables|Default|GetSphere)))
          (Utilities|IsValid (Components|GetOwner _pickup)
            (:Is%20Valid
              (bind _asbp_spawnable_base (Utilities|Casting|CastToBP_SpawnableBase (Components|GetOwner _pickup)))
              (Variables|/Game/Spawnables/Base/BP_SpawnableBase.BP_SpawnableBase_C|SetLastHeldByPawn _asbp_spawnable_base self)
              (bind _asbp_top_down_controller (Utilities|Casting|CastToBP_TopDownController (Pawn|GetController)))
              (Variables|/Game/Spawnables/Base/BP_SpawnableBase.BP_SpawnableBase_C|SetLastHeldByController _asbp_spawnable_base _asbp_top_down_controller))))))))

(event Input|EnhancedActionEvents|EnhancedInputActionIA_Throw
  (params (ActionValue :type Boolean) (ElapsedSeconds :type Float%20%28double-precision%29) (TriggeredSeconds :type Float%20%28double-precision%29) (InputAction :type Input%20Action%20Object%20Reference :default "/Game/ThirdPerson/Input/Actions/IA_Throw.IA_Throw"))
  (bind _returnvalue (CallFunction|GetEndLocation))
  (Utilities|HasGrabbed
    (:Has%20Grabbed
      (Utilities|FlowControl|Sequence
        (:then_0
          (Animation|Montage|PlayMontage (Variables|Default|Getplayer-arms2) "/Game/Player/PlayerView/player-arms2_Anim__player_arms_arms_throw_Montage.player-arms2_Anim__player_arms_arms_throw_Montage"))
        (:then_1
          (Physics|Components|PhysicsHandle|ReleaseComponent (Variables|Default|GetPhysicsHandle))
          (Variables|Character|GetMesh
            (:then
              (bind _tossvelocity (Class|GameplayStatics|BlueprintSuggestProjectileVelocity (Transformation|GetWorldLocation (Variables|Default|GetLastGrabbed)) _returnvalue (Variables|Default|GetLaunchVelocity) 0.0 "DoNotTrace" 56.0 true false true))
              (Physics|SetPhysicsLinearVelocity (Variables|Default|GetLastGrabbed) (* _tossvelocity 2.0) false "None")
              (Rendering|Debug|DrawDebugBox _returnvalue "100.000000,100.000000,100.000000" "(R=1.000000,G=0.006644,B=0.000000,A=1.000000)" "0, 0, 0" 2.0 15.0))
            (:else)))))
    (:No%20Grabbed
      (bind _returnvalue_2 (Actor|GetActorOfClass "/Game/ImpactExecutor.ImpactExecutor_C"))
      (Default|FireImpact _returnvalue_2 (Transformation|GetActorLocation)))))

(event EventTick
  (params (DeltaSeconds :type Float%20%28single-precision%29))
  (Utilities|FlowControl|Sequence
    (:then_0
      (Utilities|HasGrabbed
        (:Has%20Grabbed
          (Physics|Components|PhysicsHandle|SetTargetLocation (Variables|Default|GetPhysicsHandle) (Transformation|GetWorldLocation (Variables|Default|GetSphere)))
          (CallFunction|SetGrabAvailableUIVisible false))))
    (:then_1
      (CallFunction|UpdateCamera))))

(event EventBeginPlay
  (bind _returnvalue (Actor|GetActorOfClass "/Game/Dumpster.Dumpster_C"))
  (Variables|Default|SetDumpster _returnvalue))

(event Input|KeyboardEvents|5
  (params (Key :type Key%20Structure))
  (:Pressed
    (Animation|Montage|PlayMontage (Variables|Default|Getplayer-arms2) "/Game/Player/PlayerView/player-arms2_Anim__player_arms_arms_celebrate_Montage.player-arms2_Anim__player_arms_arms_celebrate_Montage")))

(fn ConstructionScript)

(fn CanGrab
  (params (self2 :type Scene%20Component%20Object%20Reference))
  (return (Physics|IsSimulatingPhysics self2 "None")))

(fn GetGrabComponent
  (bind _sphere (Variables|Default|GetSphere))
  (bind _overlappingactors (Collision|GetOverlappingActors _sphere "/Game/Spawnables/Base/BP_SpawnableBase.BP_SpawnableBase_C" :!class /Script/Engine.PrimitiveComponent))
  (LocalVariables|Setclosest 1e+26)
  (if (> (Utilities|Array|Length _overlappingactors) 0)
    (for _array_element _overlappingactors
      (if (< (Math|Vector|Distance(Vector) (Transformation|GetActorLocation _array_element) (Transformation|GetActorLocation)) (LocalVariables|Getclosest))
        (LocalVariables|Setclosest (Math|Vector|Distance(Vector) (Transformation|GetActorLocation _array_element) (Transformation|GetActorLocation)))
        (LocalVariables|Setbest (Actor|GetComponentbyClass _array_element "/Script/Engine.StaticMeshComponent"))))
    (return (Utilities|IsValid (LocalVariables|Getbest)) (LocalVariables|Getbest))
    (else
      (return false 0))))

(fn SetGrabAvailableUIVisible
  (params (bNewVisibility :type Boolean))
  (Rendering|SetVisibility (Variables|Default|GetSphere1) bNewVisibility false))

(fn UpdateCamera
  (bind _outactors (Actor|GetAllActorsOfClass "BP_PlayerBear_C"))
  (Utilities|FlowControl|Sequence
    (:then_0
      (for _array_element _outactors
        (LocalVariables|Setsum (+ (Transformation|GetActorLocation _array_element) (LocalVariables|Getsum)))))
    (:then_2
      (bind _returnvalue (Actor|GetActorOfClass "/Game/Player/Blueprints/BP_Camera.BP_Camera_C"))
      (Transformation|SetWorldLocation (Variables|Default|GetCameraParent) (Transformation|GetActorLocation _returnvalue) false false)
      (bind _returnvalue_2 (Actor|GetActorOfClass "/Game/Player/Blueprints/BP_CameraTarget.BP_CameraTarget_C"))
      (Transformation|SetWorldRotation (Variables|Default|GetCameraParent) (Math|Rotator|FindLookatRotation (Transformation|GetActorLocation _returnvalue) (Transformation|GetActorLocation _returnvalue_2)) false false)
      (Transformation|SetWorldRotation (Variables|Default|GetbodyPivot) (Math|Rotator|FindLookatRotation (Transformation|GetActorLocation _returnvalue) (Transformation|GetActorLocation _returnvalue_2)) false false)
      (Transformation|SetActorRotation _returnvalue (Math|Rotator|FindLookatRotation (Transformation|GetActorLocation _returnvalue) (Transformation|GetActorLocation _returnvalue_2))))))

(fn GetEndLocation
  (bind _mesh (Variables|Character|GetMesh))
  (bind _returnvalue (Math|Vector|GetRightVector _mesh))
  (LocalVariables|SetDumpsterLocation (Transformation|GetActorLocation (Variables|Default|GetDumpster)))
  (if (< (Math|Vector|Distance2D(Vector) (Transformation|GetActorLocation) (LocalVariables|GetDumpsterLocation)) 5e+02)
    _
    (elif (> (Math|Vector|DotProduct _returnvalue (Math|Vector|Normalize (* (- (LocalVariables|GetDumpsterLocation) (Transformation|GetActorLocation)) "1.000000,1.000000,0.000000"))) 0.5)
      _
      (else
        (return (+ (Transformation|GetActorLocation) (* _returnvalue 1.5e+03))))))
  (return (LocalVariables|GetDumpsterLocation)))