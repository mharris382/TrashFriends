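; BP_StartMenuButton is an in-world start menu button actor that shows its current button state visually.
; ChangeState stores the new state and shows only the matching default, hover or pressed mesh among separately referenced mesh actors.
; It also shows a text-render cursor actor for any non-default state.
; BeginPlay applies the initial state and hides the cursor; input and click handling are not in this Blueprint.
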(event EventBeginPlay
  (bind _cursor (Variables|Default|GetCursor))
  ;[0 0 0 0.5 60] Begin Play
  (CallFunction|ChangeState (Variables|Default|GetState))
  (Utilities|IsValid _cursor
    (:Is%20Valid
      (Rendering|SetVisibility (Variables|/Script/Engine.TextRenderActor|GetTextRender _cursor) false false))))

(event Collision|EventActorBeginOverlap
  (params (OtherActor :type Actor%20Object%20Reference)))

(event EventTick
  (params (DeltaSeconds :type Float%20%28single-precision%29)))

(fn ConstructionScript)

(fn ChangeState
  (params (New%20State :type ButtonState%20Enum :default "NewEnumerator0"))
  (bind _mesh_default (Variables|Default|GetMesh%20Default))
  (bind _cursor (Variables|Default|GetCursor))
  (bind _mesh_hover (Variables|Default|GetMesh%20Hover))
  (bind _mesh_pressed (Variables|Default|GetMesh%20Pressed))
  ;[0 0 0 0.5 60] Change State
  (Variables|Default|SetState New%20State)
  (Utilities|FlowControl|Sequence
    (:then_0
      ;;[0.15 0.15 0.15 0.5 40] set visibility for default mesh
      (Utilities|IsValid _mesh_default
        (:Is%20Valid
          (Rendering|SetVisibility (Variables|/Script/Engine.StaticMeshActor|GetStaticMeshComponent _mesh_default) (Utilities|Enum|Equal(Enum) (Variables|Default|GetState) "NewEnumerator0") false))
        (:Is%20Not%20Valid
          _))
      ;;[0.15 0.15 0.15 0.5 40] hover mesh
      (Utilities|IsValid _mesh_hover
        (:Is%20Valid
          (Rendering|SetVisibility (Variables|/Script/Engine.Actor|GetRootComponent _mesh_hover) (Utilities|Enum|Equal(Enum) (Variables|Default|GetState) "NewEnumerator1") false))
        (:Is%20Not%20Valid
          _))
      ;;[0.15 0.15 0.15 0.5 40] pressed
      (Utilities|IsValid _mesh_pressed
        (:Is%20Valid
          (Rendering|SetVisibility (Variables|/Script/Engine.Actor|GetRootComponent _mesh_pressed) (Utilities|Enum|Equal(Enum) (Variables|Default|GetState) "NewEnumerator2") false))))
    (:then_1
      ;;[0.15 0.15 0.15 0.5 40] Cursor visible on hover or pressed
      (Utilities|IsValid _cursor
        (:Is%20Valid
          (Rendering|SetVisibility (Variables|/Script/Engine.TextRenderActor|GetTextRender _cursor) (!= (Variables|Default|GetState) (Class|KismetMathLibrary|ToInt64(Byte) (Utilities|Enum|LiteralenumButtonState "NewEnumerator0"))) false))))))