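; BP_GameCamera is the game's roaming camera, which mirrors placed title, start menu, gameplay, results and credits cameras.
; BeginPlay finds one actor of each class and maps it to an enum key.
; AnimateTo starts a one-second linear blend of transform and FOV to the chosen camera, promoting any pending target first, and prints a debug stack trace.
; Tick drives the blend, otherwise tracks the current camera.
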(event EventBeginPlay
  ;[0.15 0.15 0.15 0.5] Find Title Camera
  (bind _returnvalue (Actor|GetActorOfClass "/Game/GameLoop/BP_TitleCamera.BP_TitleCamera_C"))
  (Utilities|Map|Add (Variables|Default|Getall_cameras) "NewEnumerator0" _returnvalue)
  ;[0.15 0.15 0.15 0.5] Find Start Menu Camera
  (bind _returnvalue_2 (Actor|GetActorOfClass "/Game/GameLoop/BP_StartMenuCamera.BP_StartMenuCamera_C"))
  (Utilities|Map|Add (Variables|Default|Getall_cameras) "NewEnumerator1" _returnvalue_2)
  ;[0.15 0.15 0.15 0.5] Find the first Game Camera
  (bind _returnvalue_3 (Actor|GetActorOfClass "/Game/GameLoop/BP_GameplayCamera.BP_GameplayCamera_C"))
  (Utilities|Map|Add (Variables|Default|Getall_cameras) "NewEnumerator3" _returnvalue_3)
  ;[0.15 0.15 0.15 0.5] Find Results Cam
  (bind _returnvalue_4 (Actor|GetActorOfClass "/Game/GameLoop/BP_ResultsCamera.BP_ResultsCamera_C"))
  (Utilities|Map|Add (Variables|Default|Getall_cameras) "NewEnumerator4" _returnvalue_4)
  ;[0.15 0.15 0.15 0.5] Find Credits Cam
  (bind _returnvalue_5 (Actor|GetActorOfClass "/Game/GameLoop/BP_CreditsCamera.BP_CreditsCamera_C"))
  (Utilities|Map|Add (Variables|Default|Getall_cameras) "NewEnumerator5" _returnvalue_5))

(event EventTick
  (params (DeltaSeconds :type Float%20%28single-precision%29))
  ;[0 0 0 0.5 90] Event Tick
  (if (> (Variables|Default|GetlocalTime) 0.0)
    ;[0 0 0 0.5 60] Increment Time
    (bind _output_get (Variables|Default|SetlocalTime (- (Variables|Default|GetlocalTime) DeltaSeconds)))
    (if (<= _output_get 0.0)
      ;[0 0 0 0.5 40] Animation. finish
      ;;[0.15 0.15 0.15 0.5] store next as this and reset next. reset time
      (Variables|Default|SetthisCamera (Variables|Default|GetnextCamera))
      (Variables|Default|SetnextCamera 0)
      (Variables|Default|SetlocalTime 0.0)
      ;;[0.15 0.15 0.15 0.5] set position
      (Transformation|SetActorTransform (Transformation|GetActorTransform (Variables|Default|GetthisCamera)))
      ;;[0.15 0.15 0.15 0.5] field of view
      (Camera|SetFieldOfView (Variables|CameraActor|GetCameraComponent) (Variables|/Script/Engine.CameraComponent|GetFieldOfView (Actor|GetComponentbyClass (Variables|Default|GetthisCamera) "/Script/Engine.CameraComponent")))
      (else
        ;[0 0 0 0.5 40] Animation. continue
        (Variables|Default|GetnextCamera
          (:then
            ;;[0.15 0.15 0.15 0.5] position
            (Transformation|SetActorTransform (Math|Transform|Lerp(Transform) (Transformation|GetActorTransform (Variables|Default|GetnextCamera)) (Transformation|GetActorTransform (Variables|Default|GetthisCamera)) (Variables|Default|GetlocalTime)))
            ;;[0.15 0.15 0.15 0.5] field of view
            (bind _cameracomponent (Variables|CameraActor|GetCameraComponent)
              (:then
                (Camera|SetFieldOfView _cameracomponent (Math|Float|Lerp (Variables|/Script/Engine.CameraComponent|GetFieldOfView (Actor|GetComponentbyClass (Variables|Default|GetnextCamera) "/Script/Engine.CameraComponent")) (Variables|/Script/Engine.CameraComponent|GetFieldOfView (Actor|GetComponentbyClass (Variables|Default|GetthisCamera) "/Script/Engine.CameraComponent")) (Variables|Default|GetlocalTime))))
              (:else)))
          (:else))))
    (else
      ;[0 0 0 0.5 60] No animation. track thisCamera only
      (Transformation|SetActorTransform (Transformation|GetActorTransform (Variables|Default|GetthisCamera)))
      (Camera|SetFieldOfView (Variables|CameraActor|GetCameraComponent) (Variables|/Script/Engine.CameraComponent|GetFieldOfView (Actor|GetComponentbyClass (Variables|Default|GetthisCamera) "/Script/Engine.CameraComponent"))))))

(fn ConstructionScript)

(fn Animateto
  (params (To :type CameraPosition%20Enum :default "NewEnumerator0"))
  (bind _all_cameras (Variables|Default|Getall_cameras))
  (bind (_value _returnvalue) (Utilities|Map|Find _all_cameras To))
  ;[0.15 0.15 0.15 0.5 26] if there's an animation running, jump to the end and start this new one
  (if (Utilities|IsValid (Variables|Default|GetnextCamera))
    (Variables|Default|SetthisCamera (Variables|Default|GetnextCamera)))
  ;[0.15 0.15 0.15 0.5 26] find camera, store as next
  (if _returnvalue
    (Variables|Default|SetnextCamera _value)
    ;[0.15 0.15 0.15 0.5 26] local time counts from 1.0 to zero
    (Variables|Default|SetlocalTime 1.0)
    (Class|KismetSystemLibrary|StackTrace)
    (Development|PrintString "see stack trace")))