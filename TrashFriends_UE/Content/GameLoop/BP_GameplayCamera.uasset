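; BP_GameplayCamera is a gameplay camera actor that drifts gently around the transform it is placed at.
; BeginPlay stores that starting transform, and Tick accumulates local time and rebuilds the actor transform from it each frame.
; Time-driven Perlin noise offsets position and roll, while a slow sine wave adds horizontal sway along Y; pitch, yaw and scale stay fixed.
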(event EventBeginPlay
  ;[0 0 0 0.5 40] BeginPlay
  (Variables|Default|Setstarting_position (Transformation|GetActorTransform)))

(event EventTick
  (params (DeltaSeconds :type Float%20%28single-precision%29))
  (bind _starting_position (Variables|Default|Getstarting_position))
  (bind (_location _rotation _scale) (Math|Transform|BreakTransform _starting_position))
  (bind (_roll _pitch _yaw) (Math|Rotator|BreakRotator _rotation))
  ;[0 0 0 0.5 40] increment local time
  (Variables|Default|SetlocalTime (+ DeltaSeconds (Variables|Default|GetlocalTime)))
  (Transformation|SetActorTransform (Math|Transform|MakeTransform (Math|Vector|MakeVector (.X (Math|Vector|BreakVector (+ (Class|KismetAnimationLibrary|MakePerlinNoiseVectorandRemap (* (Variables|Default|GetlocalTime) 0.083333) 0.0 0.0 0.0 65.0 "-1.f" "1.f" "-1.f" "1.f") _location))) (+ (.Y (Math|Vector|BreakVector (+ (Class|KismetAnimationLibrary|MakePerlinNoiseVectorandRemap (* (Variables|Default|GetlocalTime) 0.083333) 0.0 0.0 0.0 65.0 "-1.f" "1.f" "-1.f" "1.f") _location))) (* (Math|Trig|Sin(Radians) (* (Variables|Default|GetlocalTime) 0.1)) 6e+01)) (.Z (Math|Vector|BreakVector (+ (Class|KismetAnimationLibrary|MakePerlinNoiseVectorandRemap (* (Variables|Default|GetlocalTime) 0.083333) 0.0 0.0 0.0 65.0 "-1.f" "1.f" "-1.f" "1.f") _location)))) (Math|Rotator|MakeRotator (+ _roll (.Y (Math|Vector|BreakVector (Class|KismetAnimationLibrary|MakePerlinNoiseVectorandRemap 0.0 (* (Variables|Default|GetlocalTime) 0.142857) 0.0 0.0 65.0 "-1.f" "1.f" "-1.f" "1.f")))) _pitch _yaw) _scale)))

(fn ConstructionScript)