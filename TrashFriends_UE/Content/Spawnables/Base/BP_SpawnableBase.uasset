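; Base Blueprint for spawnable physics items that can be dumped for points in the Trash Friends game.
; Construction sets the mesh to the last RandomMesh entry, despite the function's random-pick name.
; BeginPlay plays optional effects, then launches the mesh next tick with a randomized forward impulse.
; Destruction replays those spawn effects, awards any point value to the last holding controller, and notifies the game mode.
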(event EventBeginPlay
  (bind _spawnimpulserange (Variables|Default|GetSpawnImpulseRange))
  (bind _rotaterandom (Variables|Default|GetRotateRandom))
  (bind _rotaterandom_2 (Variables|Default|GetRotateRandom))
  ;[0 0 0 0.5 60] BeginPlay
  (Utilities|FlowControl|Sequence
    (:then_1
      ;;[0.15 0.15 0.15 0.5] Spawned Effects (optional)
      (Utilities|PlayEffects (Variables|Effects|GetSpawnedVFX) (Variables|Effects|GetSpawnedSFX)))
    (:then_2
      (Utilities|FlowControl|DelayUntilNextTick)
      (Physics|AddImpulse (Variables|Default|GetStaticMesh) (* (Math|Vector|RotateVectorAroundAxis (Math|Vector|RotateVectorAroundAxis (Transformation|GetActorForwardVector) (Math|Random|RandomFloatinRange (* _rotaterandom_2 -1.0) _rotaterandom_2) (Transformation|GetActorRightVector)) (Math|Random|RandomFloatinRange (* _rotaterandom -1.0) _rotaterandom) (Transformation|GetActorUpVector)) (Math|Random|RandomFloatinRange (.x _spawnimpulserange) (.y _spawnimpulserange))) "None" true))))

(event Collision|EventActorBeginOverlap
  (params (OtherActor :type Actor%20Object%20Reference)))

(event EventTick
  (params (DeltaSeconds :type Float%20%28single-precision%29)))

(event EventDestroyed
  ;[0 0 0 0.5 60] Event Destroyed
  (Utilities|FlowControl|Sequence
    (:then_0
      ;;[0.15 0.15 0.15 0.5] Dump Effects (optional)
      (Utilities|PlayEffects (Variables|Effects|GetSpawnedVFX) (Variables|Effects|GetSpawnedSFX)))
    (:then_1
      ;;[0.15 0.15 0.15 0.5] Award Score when player dumps item (if item has value)
      (if (> (Variables|Default|GetPointValue) 0)
        (bind _lastheldbycontroller (Variables|Default|GetLastHeldByController)
          (:then
            (Default|AwardPointsfromDumpedItem _lastheldbycontroller (Variables|Default|GetPointValue) self))
          (:else))))
    (:then_2
      (bind _asbp_trash_friends_game_mode (Utilities|Casting|CastToBP_TrashFriendsGameMode (Game|GetGameMode)))
      (Default|NotifyDestroyed _asbp_trash_friends_game_mode self))))

(fn ConstructionScript
  (Utilities|PickRandomMesh))