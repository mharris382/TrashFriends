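; Game mode for Trash Friends that spawns items from level tubes and ends spawning when a local player reaches 21 points.
; A delayed loop picks a random free tube and a spawnable via cumulative weights built from class defaults, up to a live-item cap.
; A vector curve keyed on live count over the cap sets random delay bounds.
; It also animates the game camera at startup, on state changes and on a win.
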(event Custom|BeginSpawning
  ;[0 0 0 0.5 60] Spawn Loop
  (bind _time (CallFunction|GetTimetoNextSpawn :!label _label))
  (Utilities|FlowControl|Delay _time)
  (if (< (Variables|Internal|GetCurrentLiveItemCount) (Variables|Default|GetMaxLiveItemCount))
    (bind (_valid _tube) (CallFunction|GetNextTube))
    (if _valid
      (bind _spawnable (CallFunction|GetNextSpawnable))
      (Default|SpawnItemfrom _tube _spawnable)
      (Variables|Internal|SetCurrentLiveItemCount (+ (Variables|Internal|GetCurrentLiveItemCount) 1))
      (bind _winoccuredd (CallFunction|CheckforWin))
      (if _winoccuredd
        (CallFunction|TriggerWin)
        (else
          (goto _label)))
      (else
        (goto _label)))
    (else
      (goto _label))))

(event Custom|NotifyDestroyed
  (params (Spawnable :type BP%20Spawnable%20Base%20Object%20Reference))
  ;[0 0 0 0.5 60] Decrement Count upon destroyed
  (Variables|Internal|SetCurrentLiveItemCount (Math|Integer|Max(Integer) (- (Variables|Internal|GetCurrentLiveItemCount) 1))))

(event Custom|TriggerWin
  ;[0 0 0 0.5 60] TriggerWin
  (Default|Animateto (Variables|Default|GetGameCamera) "NewEnumerator4"))

(event EventBeginPlay
  ;[0 0 0 0.5 60] BeginPlay
  (Utilities|FlowControl|Sequence
    (:then_0
      ;;[0.15 0.15 0.15 0.5] get tubes
      (bind _outactors (Actor|GetAllActorsOfClass "/Game/Tube.Tube_C"))
      (Variables|Default|SetTubes _outactors)
      (CallFunction|SetupWeights))
    (:then_1
      ;;[0.15 0.15 0.15 0.5] initiate spawning after delay
      (Utilities|FlowControl|Delay 3.0) ; first startup delay
      (CallFunction|BeginSpawning))
    (:then_2
      ;;[0.15 0.15 0.15 0.5] find game camera
      (bind _returnvalue (Actor|GetActorOfClass "/Game/GameLoop/BP_GameCamera.BP_GameCamera_C"))
      (Variables|Default|SetGameCamera _returnvalue))
    (:then_3
      ;;[0.15 0.15 0.15 0.5] queue first game camera animation
      (Utilities|FlowControl|Delay 2.0)
      (Default|Animateto (Variables|Default|GetGameCamera) "NewEnumerator1"))))

(event EventTick
  (params (DeltaSeconds :type Float%20%28single-precision%29)))

(fn ConstructionScript
  (|CallParentFunction))

(fn SetupWeights
  (Utilities|FlowControl|Sequence
    (:then_0
      (for _array_element (Variables|Default|GetSpawnables)
        (LocalVariables|SetTotal (+ (.SpawnChanceWeight (Utilities|GetClassDefaults _array_element)) (LocalVariables|GetTotal)))))
    (:then_1
      (LocalVariables|SetPrev 0.0)
      (for (_array_element_2 _array_index) (Variables|Default|GetSpawnables)
        (bind _output_get (LocalVariables|SetPrev (+ (LocalVariables|GetPrev) (/ (.SpawnChanceWeight (Utilities|GetClassDefaults _array_element_2)) (LocalVariables|GetTotal)))))
        (Utilities|Array|Insert (Variables|Internal|GetChances) _output_get _array_index)))))

(fn GetNextSpawnable
  (bind _spawnables (Variables|Default|GetSpawnables))
  (LocalVariables|Setrand (Math|Random|RandomFloat))
  (for (_array_element _array_index) (Variables|Internal|GetChances)
    (if (< (LocalVariables|Getrand) _array_element)
      (return (Utilities|Array|Get(acopy) (Variables|Default|GetSpawnables) _array_index))))
  (return (Utilities|Array|Get(acopy) _spawnables (- (Utilities|Array|Length _spawnables) 1))))

(fn GetNextTube
  (bind _tmp (LocalVariables|Gettmp))
  (bind _returnvalue (Utilities|Array|Length _tmp))
  (Utilities|FlowControl|Sequence
    (:then_0
      (for _array_element (Variables|Default|GetTubes)
        (if (not (Variables|/Game/Tube.Tube_C|GetInUse _array_element))
          (Utilities|Array|Add (LocalVariables|Gettmp) _array_element))))
    (:then_1
      (if (> _returnvalue 0)
        (return true (Utilities|Array|Get(acopy) _tmp (Math|Random|RandomIntegerinRange 0 (- _returnvalue 1))))
        (else
          (return false 0))))))

(fn GetTimetoNextSpawn
  (bind _maxliveitemcount (Variables|Default|GetMaxLiveItemCount))
  (bind _spawnratecurve (Variables|Default|GetSpawnRateCurve))
  (bind _currentliveitemcount (Variables|Internal|GetCurrentLiveItemCount))
  (bind _returnvalue (/ _currentliveitemcount _maxliveitemcount))
  (bind _returnvalue_2 (Math|Conversions|ToFloat(Integer) _returnvalue))
  (bind _returnvalue_3 (Math|Curves|GetVectorValue _spawnratecurve _returnvalue_2))
  (bind (_x _y) (Math|Vector|BreakVector _returnvalue_3))
  (return (Math|Random|RandomFloatinRange _x _y)))

(fn CheckforWin
  (for _index (range 0 (- (Class|GameplayStatics|GetNumLocalPlayerControllers) 1))
    (bind _asbp_top_down_controller (Utilities|Casting|CastToBP_TopDownController (Game|GetPlayerController _index)))
    (if (>= (Variables|/Game/Player/Blueprints/BP_TopDownController.BP_TopDownController_C|GetTotalPoints _asbp_top_down_controller) 21)
      (return true)))
  (return false))

(fn ChangeState
  (params (to :type CameraPosition%20Enum :default "NewEnumerator0"))
  (Default|Animateto (Variables|Default|GetGameCamera) to)
  (Development|PrintString (Utilities|String|Append "BP_TrashFriendsGameMode.ChangeState(to game mode " (Utilities|String|ToString(Byte) to) ")")))